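; MyCharacter is a character Blueprint that tracks the player's health and mana.
; AnyDamage subtracts incoming damage from PlayerHealth with no clamp or death check.
; Tick calls Regen every frame, adding fixed regen amounts to mana and health while each is below its maximum, without scaling by delta time.
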(event EventTick
  (params (DeltaSeconds :type Float%20%28single-precision%29))
  (CallFunction|Regen))

(event EventAnyDamage
  (params (Damage :type Float%20%28single-precision%29) (DamageType :type Damage%20Type%20Object%20Reference) (InstigatedBy :type Controller%20Object%20Reference) (DamageCauser :type Actor%20Object%20Reference))
  (Variables|Default|Setplayer_health (- (Variables|Default|Getplayer_health) Damage)))

(fn ConstructionScript)

(fn Regen
  ;[1 1 1] Regen
  (Utilities|FlowControl|Sequence
    (:then_0
      (Math|Float|CompareFloat (Variables|Default|GetPlayer_mana) (Variables|Default|GetPlayer_max_mana)
        (:<
          (Variables|Default|SetPlayer_mana (+ (Variables|Default|GetPlayer_mana) (Variables|Default|Getmana_regen))))))
    (:then_1
      (Math|Float|CompareFloat (Variables|Default|Getplayer_health) (Variables|Default|Getplayer_max_health)
        (:<
          (Variables|Default|Setplayer_health (+ (Variables|Default|Getplayer_health) (Variables|Default|Gethealth_regen))))))))