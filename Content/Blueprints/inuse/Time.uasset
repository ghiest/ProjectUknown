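; Time Blueprint that begins setting up persistent game time through a "PermTime" save slot, but is unfinished.
; With PersistentTime at 1, Tick checks for the save until found, creating an in-memory GameData object whenever it is missing.
; The SaveGameToSlot call is disconnected, and the InitialTimeLoad branch leads to an empty sequence.
; CreateTimeFile duplicates the file check without being called here, and InitialPersistentTimeSync is empty.
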(event EventTick
  (params (DeltaSeconds :type Float%20%28single-precision%29))
  (bind _persistenttime (Variables|Settings|GetPersistentTime))
  (if (== _persistenttime 1)
    (Utilities|FlowControl|Sequence
      (:then_0
        (if (not (Variables|Runtime|GetFileCheck))
          (bind _returnvalue (SaveGame|DoesSaveGameExist "PermTime"))
          (if _returnvalue
            (Variables|Runtime|SetFileCheck true)
            (else
              (SaveGame|CreateSaveGameObject "/Game/Blueprints/inuse/GameData.GameData_C")))))
      (:then_2
        (if (Variables|Runtime|GetInitialTimeLoad)
          (Utilities|FlowControl|Sequence :!label _label))))
    (elif (== _persistenttime 0)
      (goto _label))))

(fn ConstructionScript)

(fn InitialPersistentTimeSync)

(fn CreateTimeFile
  (if (not (Variables|Runtime|GetFileCheck))
    (bind _returnvalue (SaveGame|DoesSaveGameExist "PermTime"))
    (if _returnvalue
      (Variables|Runtime|SetFileCheck true)
      (else
        (SaveGame|CreateSaveGameObject "/Game/Blueprints/inuse/GameData.GameData_C")))))